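; Snow-deformation capture actor that follows the player in grid-cell steps and records a scene capture into persistent render targets.
; Each tick it snaps to the player's grid cell, publishes its location to MPC_Capture and prints the cell coordinate.
; It then draws through a middle material, stamps M_DrawToPersistent onto a canvas at that cell's offset, and recaptures the scene.
; A pixel-snapped MoveCapture function exists but is not called here.
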(event `self.ReceiveBeginPlay`
  (`KismetMaterialLibrary.SetScalarParameterValue` "/Game/Carla/MyCarla/SnowDeform2/MPC_Capture.MPC_Capture" "CaptureSize" (`SceneCaptureComponent2D.OrthoWidth` (`self.SceneCapture`)))
  (bind _returnvalue (`KismetMaterialLibrary.CreateDynamicMaterialInstance` "/Game/Carla/MyCarla/SnowDeform2/M_DrawToPersistent.M_DrawToPersistent"))
  (set `self.DrawToPersistenMaterial` _returnvalue)
  (bind _returnvalue_2 (`KismetMaterialLibrary.CreateDynamicMaterialInstance` "/Game/Carla/MyCarla/SnowDeform2/M_DrawToMiddle.M_DrawToMiddle"))
  (set `self.DrawToMiddle` _returnvalue_2)
  (`KismetRenderingLibrary.ClearRenderTarget2D` null)
  (`KismetRenderingLibrary.ClearRenderTarget2D` null)
  (bind _grid (`/Game/Carla/MyCarla/SnowDeform2/ActorFinder.GetGrid`))
  (set `self.Grid` _grid))

(event `self.ReceiveTick`
  (params (DeltaSeconds :type "Float (single-precision)"))
  (bind _grid (`/Game/Carla/MyCarla/SnowDeform2/ActorFinder.GetGrid`))
  (`/Game/Carla/MyCarla/SnowDeform2/Grid.SnapActorToCoord` _grid (`self.K2_GetActorLocation` (`GameplayStatics.GetPlayerPawn` 0)) self)
  (`KismetMaterialLibrary.SetVectorParameterValue` "/Game/Carla/MyCarla/SnowDeform2/MPC_Capture.MPC_Capture" "CaptureLocation" (`KismetMathLibrary.Conv_VectorToLinearColor` (`self.K2_GetActorLocation`)))
  (`self.DrawToPersistent`)
  (bind (_x _y) (`/Game/Carla/MyCarla/SnowDeform2/Grid.LocationToCoord` _grid (`self.K2_GetActorLocation`)))
  (`KismetSystemLibrary.PrintString` (`KismetTextLibrary.Conv_TextToString` (`|FormatText` "{x} {y}" _x _y))))

(fn `DrawToPersistent`
  (bind _grid (`self.Grid`))
  (bind _drawtomiddle (`self.DrawToMiddle`))
  (bind _grid_2 (`self.Grid`))
  (bind _returnvalue (`KismetMathLibrary.Conv_IntToDouble` (`/Game/Carla/MyCarla/SnowDeform2/Grid.CeilSize` _grid)))
  (bind (_returnvalue_x _returnvalue_y) (`KismetMathLibrary.BreakVector2D` (/ (`self.MoveOffset`) (`SceneCaptureComponent2D.OrthoWidth` (`self.SceneCapture`)))))
  (bind _returnvalue_2 (/ (`KismetMathLibrary.Conv_IntToDouble` (`/Game/Carla/MyCarla/SnowDeform2/Grid.CeilSize` _grid_2)) (`KismetMathLibrary.Conv_IntToDouble` (`/Game/Carla/MyCarla/SnowDeform2/Grid.GridSize` _grid_2))))
  (`MaterialInstanceDynamic.SetScalarParameterValue` _drawtomiddle "TileX" _returnvalue_2)
  (`MaterialInstanceDynamic.SetScalarParameterValue` _drawtomiddle "TileY" _returnvalue_2)
  (`MaterialInstanceDynamic.SetVectorParameterValue` (`self.DrawToMiddle`) "Offset" (make `LinearColor` _returnvalue_x _returnvalue_y 0.0 1.0))
  (`MaterialInstanceDynamic.SetVectorParameterValue` (`self.DrawToPersistenMaterial`) "Offset" (make `LinearColor` _returnvalue_x _returnvalue_y 0.0 1.0))
  (`KismetRenderingLibrary.DrawMaterialToRenderTarget` null (`self.DrawToMiddle`))
  (bind (_canvas _size _context) (`KismetRenderingLibrary.BeginDrawCanvasToRenderTarget` null))
  (bind (_x _y) (`/Game/Carla/MyCarla/SnowDeform2/Grid.LocationToCoord` _grid (`self.K2_GetActorLocation`)))
  (bind (_x_2 _y_2) (`KismetMathLibrary.BreakVector2D` (/ _size 1.0)))
  (`Canvas.K2_DrawMaterial` _canvas "/Game/Carla/MyCarla/SnowDeform2/M_DrawToPersistent.M_DrawToPersistent" (`KismetMathLibrary.MakeVector2D` (* _x _returnvalue) (* _y _returnvalue)) (`KismetMathLibrary.MakeVector2D` _x_2 _y_2) (0.0 0.0) (1.0 1.0) 0.0 (0.5 0.5))
  (`KismetRenderingLibrary.EndDrawCanvasToRenderTarget` _context)
  (`SceneCaptureComponent2D.CaptureScene` (`self.SceneCapture`)))

(fn `MoveCapture`
  (bind (_returnvalue_x _returnvalue_y) (`KismetMathLibrary.BreakVector` (`self.K2_GetActorLocation` (`GameplayStatics.GetPlayerCharacter` 0))))
  (bind (_returnvalue_x_2 _returnvalue_y_2) (`KismetMathLibrary.BreakVector` (- (`self.SnapToPixelWorldSize` _returnvalue_x _returnvalue_y (* (`SceneCaptureComponent2D.OrthoWidth` (`self.SceneCapture`)) (/ 1.0 1.0))) (`self.K2_GetActorLocation`))))
  (bind _output_get (set `self.MoveOffset` (`KismetMathLibrary.MakeVector2D` _returnvalue_x_2 _returnvalue_y_2)))
  (`self.K2_AddActorWorldOffset` (`KismetMathLibrary.MakeVector` (`KismetMathLibrary.BreakVector2D` _output_get) (`.Y` (`KismetMathLibrary.BreakVector2D` _output_get))))
  (`KismetMaterialLibrary.SetVectorParameterValue` "/Game/Carla/MyCarla/SnowDeform2/MPC_Capture.MPC_Capture" "CaptureLocation" (`KismetMathLibrary.Conv_VectorToLinearColor` (`self.K2_GetActorLocation`))))

(fn `UserConstructionScript`)
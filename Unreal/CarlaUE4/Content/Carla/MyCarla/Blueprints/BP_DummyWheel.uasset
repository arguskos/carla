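; BP_DummyWheel is a cylinder-based dummy wheel actor that hides itself from a Carla scene capture sensor.
; On BeginPlay it zeroes the cylinder's custom depth stencil, then a one-second timer calls DoBullshit to add the actor to the first found SceneCaptureSensor's hidden list.
; SetScaleBasedOnSpeed derives X and Y scale from absolute speed, but equal clamp bounds pin both to one while Z is kept.
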(event `self.ReceiveBeginPlay`
  (`PrimitiveComponent.SetCustomDepthStencilValue` (`self.Cylinder`) 0)
  (`KismetSystemLibrary.K2_SetTimer` null "DoBullshit" 1.0))

(event `self.ReceiveTick`
  (params (DeltaSeconds :type "Float (single-precision)")))

(fn `DoBullshit`
  (bind _returnvalue (`GameplayStatics.GetActorOfClass` "/Script/Carla.SceneCaptureSensor"))
  (`SceneCaptureSensor.AddActorToHidden` _returnvalue self))

(fn `SetScaleBasedOnSpeed`
  (params (Speed :type "Float (double-precision)"))
  (bind _cylinder (`self.Cylinder`))
  (bind (_relativescale3d_x _relativescale3d_y _relativescale3d_z) (`KismetMathLibrary.BreakVector` (`SceneComponent.RelativeScale3D` _cylinder)))
  (bind _returnvalue (`KismetMathLibrary.FClamp` (/ (`KismetMathLibrary.Abs` Speed) 1500.0) 1.0 1.0))
  (`SceneComponent.SetRelativeScale3D` _cylinder (`KismetMathLibrary.MakeVector` _returnvalue _returnvalue _relativescale3d_z)))

(fn `UserConstructionScript`)
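; Test capture actor that accumulates top-level render-target data for listed actors across a grid, following CenterActor's cell.
; A show-only orthographic scene capture snaps to that cell and captures each tick.
; Canvas drawing stamps a material into the matching region of a larger persistent target.
; A post-process material receives that region's UV and scale to write back into the capture, while MPC_Capture holds capture location and size.
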(event `self.ReceiveBeginPlay`
  (set `self.BigRTSize` (`KismetMathLibrary.Conv_IntToDouble` (`TextureRenderTarget2D.SizeX` (`self.FinalRenderTarget`))))
  (set `self.SmallRTSize` (`KismetMathLibrary.Conv_IntToDouble` (`TextureRenderTarget2D.SizeX` (`self.SmallRenderTarget`))))
  (`KismetRenderingLibrary.ClearRenderTarget2D` "/Game/Carla/MyCarla/SnowDeform2/FinalTestRenderTarget.FinalTestRenderTarget")
  (`KismetRenderingLibrary.ClearRenderTarget2D` "/Game/Carla/MyCarla/SnowDeform2/SmallRenderTarget.SmallRenderTarget")
  (bind _grid (`/Game/Carla/MyCarla/Blueprints/ActorFinder.GetGrid`))
  (bind _output_get (set `self.Grid` _grid))
  (bind _output_get_2 (set `self.CellSize` (`KismetMathLibrary.FTrunc` (* (`self.SmallRTSize`) (`KismetMathLibrary.Conv_IntToDouble` (`self.UnitsPerPiexel`))))))
  (`/Game/Carla/MyCarla/Blueprints/Capture/Grid.Init` _output_get _output_get_2)
  (bind _returnvalue (`KismetMaterialLibrary.CreateDynamicMaterialInstance` "/Game/Carla/MyCarla/SnowDeform2/PP_WriteBackToCapture.PP_WriteBackToCapture"))
  (set `SceneCaptureComponent2D.PostProcessSettings` (make `PostProcessSettings` :`WeightedBlendables` (make `WeightedBlendables` (`|MakeArray` (make `WeightedBlendable` 1.0 _returnvalue) :!type "WeightedBlendable Structure"))) (`self.SceneCaptureComponent2D`))
  (set `self.PP_CaptureOverwrite` _returnvalue)
  (`self.SetupCaptureSize`)
  (for _array_element (`self.IncludeToCaptureActors`)
    (`self.AddActorToCapture` _array_element)
    (`KismetMaterialLibrary.SetVectorParameterValue` "/Game/Carla/MyCarla/SnowDeform2/MPC_Capture.MPC_Capture" "CaptureLocation" (`KismetMathLibrary.Conv_VectorToLinearColor` (`/Game/Carla/MyCarla/Blueprints/Capture/Grid.Offset` (`self.Grid`))))))

(event `self.ReceiveTick`
  (params (DeltaSeconds :type "Float (single-precision)"))
  (bind (_x _y) (`self.GetActorCoordinate`))
  ;[1 1 1] Dont draw first frame of new cell because of ghost objects
  (if (and (== (`self.LastX`) _x) (== _y (`self.LastY`)))
    (if (`self.dontCapture`)
      (set `self.dontCapture` false)
      (`KismetRenderingLibrary.ClearRenderTarget2D` (`self.SmallRenderTarget`))
      (`self.MoveCapture`)
      (else
        (`|ExecutionSequence`
          (:`then_3`
            (bind (_out_x _out_y) (`self.GetPositionOnCanvas` (stale _outx) (stale _outy) :!label _label))
            (bind (_u _v) (`self.ToUV` _out_y _out_x (`self.BigRTSize`)))
            (`self.DrawToPersistent` _out_x _out_y (`self.SmallRTSize`))
            (`self.PostProcessCaptureOverwrite` (`self.GerRatio`) _u _v))
          (:`then_5`
            (set `self.LastX` _x :!label _label_2)
            (set `self.LastY` _y)
            (`SceneCaptureComponent2D.CaptureScene` (`self.SceneCaptureComponent2D`))))))
    (else
      (`|ExecutionSequence`
        (:`then_0`
          (`self.MoveCapture`)
          (bind (_outx _outy) (`self.IndexToDrawCenter` _y _x))
          (goto _label))
        (:`then_1`
          (goto _label_2))))))

(fn `AddActorsToCapture`
  (params (Actors :type "Array of Actor Object Reference"))
  (for _array_element Actors
    (`self.AddActorToCapture` _array_element)))

(fn `AddActorToCapture`
  (params (Actor :type "Actor Object Reference"))
  (`SceneCaptureComponent.ShowOnlyActorComponents` (`self.SceneCaptureComponent2D`) Actor))

(fn `ClearTarget`
  (params (X :type Integer) (Y :type Integer))
  (bind _lastx (`self.LastX`))
  (bind _lasty (`self.LastY`))
  (if (or (!= X _lastx) (!= Y _lasty))
    (`KismetSystemLibrary.PrintString` "clear")
    (`KismetRenderingLibrary.ClearRenderTarget2D` (`self.SmallRenderTarget`))
    (else
      (`KismetSystemLibrary.PrintString` (`KismetTextLibrary.Conv_TextToString` (`|FormatText` "cur X:{X} old X:{_oldx}, cur Y: {Y} old Y:{_oldY}" X _lastx Y _lasty)) true true (struct :`R` 1.0 :`B` 0.085927 :`A` 1.0)))))

(fn `DrawToPersistent`
  (params (ScreenCenterX :type "Float (double-precision)") (ScreenCenterY :type "Float (double-precision)") (SmallSize :type "Float (double-precision)"))
  (locals (L_SmallSize :type "Float (double-precision)"))
  (bind (_canvas _size _context) (`KismetRenderingLibrary.BeginDrawCanvasToRenderTarget` "/Game/Carla/MyCarla/SnowDeform2/FinalTestRenderTarget.FinalTestRenderTarget"))
  (`Canvas.K2_DrawMaterial` _canvas "/Game/Carla/MyCarla/SnowDeform2/WriteToMiddleNoAdditive.WriteToMiddleNoAdditive" (`KismetMathLibrary.MakeVector2D` ScreenCenterX ScreenCenterY) (`KismetMathLibrary.MakeVector2D` SmallSize SmallSize) (0.0 0.0) (1.0 1.0) 0.0 (0.5 0.5))
  (`KismetRenderingLibrary.EndDrawCanvasToRenderTarget` _context))

(fn `GetActorCoordinate`
  (returns (X :type Integer) (Y :type Integer))
  (bind (_x _y) (`/Game/Carla/MyCarla/Blueprints/Capture/Grid.LocationToCoord` (`self.Grid`) (`self.K2_GetActorLocation` (`self.CenterActor`))))
  (if (`self.DebugPrintCoord`)
    (`KismetSystemLibrary.PrintString` (`KismetTextLibrary.Conv_TextToString` (`|FormatText` "{x} {y}" _x _y))))
  (return _x _y))

(fn `GetPositionOnCanvas`
  (params (X :type "Float (double-precision)") (Y :type "Float (double-precision)"))
  (returns (Out_X :type "Float (double-precision)") (Out_Y :type "Float (double-precision)"))
  (bind _returnvalue (/ (`self.SmallRTSize`) 2.0))
  (return (- X _returnvalue) (- Y _returnvalue)))

(fn `IndexToDrawCenter`
  (params (InX :type Integer) (InY :type Integer))
  (returns (OutX :type "Float (double-precision)") (OutY :type "Float (double-precision)"))
  (bind _returnvalue (/ (`self.BigRTSize`) 2.0))
  (bind _returnvalue_2 (/ (`/Game/Carla/MyCarla/Blueprints/Capture/Grid.Width` (`self.Grid`)) 2))
  (bind (_x _y) (`KismetMathLibrary.BreakVector2D` (`KismetMathLibrary.MakeVector2D` (+ (* (- InY _returnvalue_2) (* (`self.SmallRTSize`) -1.0)) _returnvalue) (+ (* (- InX _returnvalue_2) (`self.SmallRTSize`)) _returnvalue))))
  (return _x _y))

(fn `MoveCapture`
  (`/Game/Carla/MyCarla/Blueprints/Capture/Grid.SnapActorToCoord` (`self.Grid`) (`self.K2_GetActorLocation` (`self.CenterActor`)) self))

(fn `PostProcessCaptureOverwrite`
  (params (Scale :type "Float (double-precision)") (U :type "Float (double-precision)") (V :type "Float (double-precision)"))
  (bind _pp_captureoverwrite (`self.PP_CaptureOverwrite`))
  (`MaterialInstanceDynamic.SetScalarParameterValue` _pp_captureoverwrite "Scale" Scale)
  (`MaterialInstanceDynamic.SetScalarParameterValue` _pp_captureoverwrite "U" U)
  (`MaterialInstanceDynamic.SetScalarParameterValue` _pp_captureoverwrite "V" V))

(fn `SetupCaptureSize`
  (set `SceneCaptureComponent2D.OrthoWidth` (`KismetMathLibrary.Conv_IntToDouble` (`/Game/Carla/MyCarla/Blueprints/Capture/Grid.CeilSize` (`self.Grid`))) (`self.SceneCaptureComponent2D`))
  (`KismetMaterialLibrary.SetScalarParameterValue` "/Game/Carla/MyCarla/SnowDeform2/MPC_Capture.MPC_Capture" "CaptureSize" (* (`SceneCaptureComponent2D.OrthoWidth` (`self.SceneCaptureComponent2D`)) (/ (`self.BigRTSize`) (`self.SmallRTSize`)))))

(fn `ToUV`
  (params (Y :type "Float (double-precision)") (X :type "Float (double-precision)") (BigSize :type "Float (double-precision)"))
  (returns (U :type "Float (double-precision)") (V :type "Float (double-precision)"))
  (return (/ X BigSize) (/ Y BigSize)))

(fn `UserConstructionScript`)
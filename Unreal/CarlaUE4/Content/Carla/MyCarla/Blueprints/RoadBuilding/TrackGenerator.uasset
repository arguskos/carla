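; Track generator actor that builds a looping road mesh along a spline, optionally shaped from points read from a named file and scaled by 100.
; Construction script and BeginPlay size per-point RoadData to the spline, then add one spline mesh per point, wrapping last to first.
; RoadData sets each segment's banking, width and thickness.
; Pressing D appends world-space samples along the spline to Points and writes them to outpath.txt.
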(event `self.ReceiveBeginPlay`
  (if (`self.PointsFromFile`)
    (bind _returnvalue (`FIlesMisc.Read` (`self.name`)))
    (set `self.points` _returnvalue)
    (`KismetSystemLibrary.PrintString` (`KismetStringLibrary.Conv_IntToString` (`KismetArrayLibrary.Array_Length` _returnvalue)))
    (`self.MakeFromPoints` _returnvalue))
  (`self.Contstruct`)
  (`self.EnableInput` (`GameplayStatics.GetPlayerController` 0)))

(event `Key|D`
  (params (Key :type "Key Structure"))
  (:`Pressed`
    (`self.WritePoints`)))

(fn `BuildTrackElement`
  (params (TrackElement :type "StaticMesh Object Reference") (LoopIndex :type Integer))
  (locals (CurrentLoopIndex :type Integer) (NextLoopIndex :type Integer) (MeshElement :type "StaticMesh Object Reference") (StartLocation :type "Vector Structure") (EndLocation :type "Vector Structure") (StartTangent :type "Vector Structure") (EndTangent :type "Vector Structure") (CurrentSplineMesh :type "SplineMeshComponent Object Reference") (LStartRoll :type "Float (double-precision)") (LEndRoll :type "Float (double-precision)") (LStartScale :type "Vector2D Structure") (LEndScale :type "Vector2D Structure"))
  (bind _roaddata (`self.RoadData`))
  (bind _currentsplinemesh (`local.CurrentSplineMesh`))
  (bind (_location _tangent) (`SplineComponent.GetLocationAndTangentAtSplinePoint` (`self.Spline`) (`local.NextLoopIndex`) "Local"))
  (bind (_location_2 _tangent_2) (`SplineComponent.GetLocationAndTangentAtSplinePoint` (`self.Spline`) (`local.CurrentLoopIndex`) "Local"))
  (bind (_leftguard _rightguard _tackbank _width _thikness) (break `/Game/Carla/Blueprints/MyCarla/RoadBuilding/RoadData` (`|GetArrayItem` _roaddata (`local.NextLoopIndex`))))
  (bind (_leftguard_2 _rightguard_2 _tackbank_2 _width_2 _thikness_2) (break `/Game/Carla/Blueprints/MyCarla/RoadBuilding/RoadData` (`|GetArrayItem` _roaddata (`local.CurrentLoopIndex`))))
  (set `local.CurrentLoopIndex` LoopIndex)
  (set `local.NextLoopIndex` (mod (+ LoopIndex 1) (`self.NumberOfPoints`)))
  (set `local.MeshElement` TrackElement)
  (`|ExecutionSequence`
    (:`then_0`
      (set `local.StartLocation` _location_2)
      (set `local.StartTangent` _tangent_2)
      (set `local.EndLocation` _location)
      (set `local.EndTangent` _tangent)
      (set `local.LStartRoll` _tackbank_2)
      (set `local.LStartScale` (`KismetMathLibrary.MakeVector2D` _width_2 _thikness_2))
      (set `local.LEndRoll` _tackbank)
      (set `local.LEndScale` (`KismetMathLibrary.MakeVector2D` _width _thikness)))
    (:`then_1`
      (bind _returnvalue (`AddComponent|NODE_AddSplineMeshComponent-0`))
      (bind _output_get (set `local.CurrentSplineMesh` _returnvalue))
      (`StaticMeshComponent.SetStaticMesh` _output_get (`local.MeshElement`))
      (`SplineMeshComponent.SetStartAndEnd` (`local.CurrentSplineMesh`) (`local.StartLocation`) (`local.StartTangent`) (`local.EndLocation`) (`local.EndTangent`) true)
      (`SplineMeshComponent.SetStartRoll` _currentsplinemesh (`local.LStartRoll`) true)
      (`SplineMeshComponent.SetEndRoll` _currentsplinemesh (`local.LEndRoll`) true)
      (`SplineMeshComponent.SetStartScale` _currentsplinemesh (`local.LStartScale`) true)
      (`SplineMeshComponent.SetEndScale` _currentsplinemesh (`local.LEndScale`) true))))

(fn `Contstruct`
  (locals (NewLocalVar_0 :type "Array of /Game/Carla/Blueprints/MyCarla/RoadBuilding/RoadData Structure") (NewLocalVar_1 :type "Array of /Game/Carla/Blueprints/MyCarla/RoadBuilding/RoadData Structure") (NewLocalVar_2 :type "Array of /Game/Carla/Blueprints/MyCarla/RoadBuilding/RoadData Structure"))
  (bind _roaddata (`self.RoadData`))
  (`|ExecutionSequence`
    (:`then_0`
      (set `self.NumberOfPoints` (`SplineComponent.GetNumberOfSplinePoints` (`self.Spline`))))
    (:`then_1`
      (`/Engine/EditorBlueprintResources/StandardMacros.CompareInt` (`KismetArrayLibrary.Array_Length` _roaddata) (`self.NumberOfPoints`) :!label _label
        (:`>`
          (`KismetArrayLibrary.Array_Remove` _roaddata (`KismetArrayLibrary.Array_LastIndex` _roaddata))
          (goto _label))
        (:`<`
          (`KismetArrayLibrary.Array_Add` _roaddata)
          (goto _label))))
    (:`then_2`
      (for _index (range (`self.NumberOfPoints`))
        (`self.BuildTrackElement` (`self.RoadMesh`) _index)))))

(fn `MakeFromPoints`
  (params (Points :type "Array of Vector Structure"))
  (locals (tmpVec :type "Array of Vector Structure"))
  (for _array_element Points
    (`KismetArrayLibrary.Array_Add` (`local.tmpVec`) (* _array_element 100.0)))
  (`SplineComponent.SetSplinePoints` (`self.Spline`) (`local.tmpVec`) "Local" true))

(fn `UserConstructionScript`
  (if (`self.PointsFromFile`)
    (bind _returnvalue (`FIlesMisc.Read` (`self.name`)))
    (`self.MakeFromPoints` _returnvalue))
  (`self.Contstruct`))

(fn `WritePoints`
  (locals (Time :type "Float (double-precision)"))
  (while (<= (`local.Time`) 1.0)
    (bind _output_get (set `local.Time` (+ (`local.Time`) 0.01)))
    (`KismetArrayLibrary.Array_Add` (`self.points`) (`SplineComponent.GetLocationAtTime` (`self.Spline`) _output_get "World" false)))
  (`FIlesMisc.WritePoints` "outpath.txt" (`self.points`) "WT_Points")
  (`KismetSystemLibrary.PrintString` "wrote fil;e"))